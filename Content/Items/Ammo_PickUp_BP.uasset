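; Ammo pickup actor that refills the top-down player character's ammo when touched.
; On box overlap by that character, it plays a pickup sound, adds a random amount of ammo clamped to the character's maximum, refreshes the HUD ammo text and destroys itself.
; The overlapping actor is compared to a stored character reference, which is not assigned anywhere in these graphs.
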(event OnComponentBeginOverlap(Box)
  (params (OverlappedComponent :type Primitive%20Component%20Object%20Reference) (OtherActor :type Actor%20Object%20Reference) (OtherComp :type Primitive%20Component%20Object%20Reference) (OtherBodyIndex :type Integer) (bFromSweep :type Boolean) (SweepResult :type Hit%20Result%20Structure%20%28by%20ref%29))
  (bind _as_bp_top_down_character (Variables|Default|GetAs%20BP%20Top%20Down%20Character))
  (if (== OtherActor (Variables|Default|GetAs%20BP%20Top%20Down%20Character))
    (Audio|PlaySoundatLocation "/Game/SoundEffects/AmmoPickUp.AmmoPickUp" (Transformation|GetActorLocation) "0, 0, 0" 1.0 1.0 0.0 0 0 0 0)
    (Variables|/Game/TopDown/Blueprints/BP_TopDownCharacter.BP_TopDownCharacter_C|SetAmmo _as_bp_top_down_character (Math|Integer|Clamp(Integer) (+ (Variables|/Game/TopDown/Blueprints/BP_TopDownCharacter.BP_TopDownCharacter_C|GetAmmo _as_bp_top_down_character) (Math|Random|RandomIntegerinRange 15 25)) 0 (Variables|/Game/TopDown/Blueprints/BP_TopDownCharacter.BP_TopDownCharacter_C|GetMaxAmmo (Variables|Default|GetAs%20BP%20Top%20Down%20Character))))
    (Default|UpdateAmmoText (Variables|/Game/TopDown/Blueprints/BP_TopDownCharacter.BP_TopDownCharacter_C|GetPlayerHUDref _as_bp_top_down_character))
    (Actor|DestroyActor)))

(event EventBeginPlay
  (|CallParentFunction) ; This node is disabled and will not be called.\nDrag off pins to build functionality.
)

(event Collision|EventActorBeginOverlap
  (params (OtherActor :type Actor%20Object%20Reference))
  (|CallParentFunction OtherActor) ; This node is disabled and will not be called.\nDrag off pins to build functionality.
)

(event EventTick
  (params (DeltaSeconds :type Float%20%28single-precision%29))
  (|CallParentFunction DeltaSeconds) ; This node is disabled and will not be called.\nDrag off pins to build functionality.
)

(fn ConstructionScript
  (|CallParentFunction))